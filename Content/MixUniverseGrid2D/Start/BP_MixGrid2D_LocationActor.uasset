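; Demo actor for the MixUniverse Grid2D sample that moves around its start location with a randomized size and speed.
; On BeginPlay it caches its location, randomly scales the sphere and derives a Radius from that scale, intended for sending to Grid2D.
; A Timeline with a random play rate then sets the actor location each update from the cached position, the scaled track value and a small constant offset.
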(event EventBeginPlay
  (Utilities|FlowControl|Sequence
    (:then_0
      ;[0.04719 0.04189 0.1458] Cache location for timeline to start from
      (Variables|Default|SetCachedLocation (Transformation|GetWorldLocation (Variables|Default|GetDefaultSceneRoot)))
      ;[0.1167 0.07547 0.1354] Set world scale randomly to showcase
      ; Individual sizes
      (Transformation|SetWorldScale3D (Variables|Default|GetSphere) (Math|Conversions|ToVector(Float) (Math|Random|RandomFloatinRange 0.5 0.25)))
      ;[0.0625 0.09326 0.125] Set Radius Value Used for Sending to Grid2D
      (Variables|Default|SetRadius (* (.X (Math|Vector|BreakVector (Transformation|GetWorldScale (Variables|Default|GetSphere)))) 1e+02)))
    (:then_1
      ;[0.102 0.149 0.2] Change Playrate of timeline.
      (Components|Timeline|SetPlayRate (Variables|Default|GetTimeline) (Math|Random|RandomFloatinRange 0.5 0.25))
      ;[0.03667 0.06771 0.06691] Simple Animation
      (bind _newtrack_0 (Timeline|Timeline PlayFromStart)
        (:Update
          (Transformation|SetActorLocation (+ (Variables|Default|GetCachedLocation) (* _newtrack_0 1e+02) "1.000000,1.000000,1.500000") false false))))))

(fn ConstructionScript)